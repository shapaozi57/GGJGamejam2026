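; Movable object actor that the player shifts in fixed Distence steps along X and Y with WASD while its Place flag is false.
; Each key spawns a temporary copy of its own class one step ahead, calls the Bianjie (boundary) check, moves the actor if it passes, then destroys the copy.
; Bianjie always returns true here, so no move is actually blocked by this class.
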(event `self.ReceiveBeginPlay`
  (`parent.ReceiveBeginPlay`)
  (`self.EnableInput` (`GameplayStatics.GetPlayerController` 0)))

(event `self.ReceiveTick`
  (params (DeltaSeconds :type "Float (single-precision)")))

(event `Key|W`
  (params (Key :type "Key Structure"))
  (bind _returnvalue_location (`KismetMathLibrary.BreakTransform` (`self.GetTransform` self)))
  (:`Pressed`
    (if (not (`self.place`))
      (bind _returnvalue (`|SpawnActorFromClass` (`GameplayStatics.GetObjectClass` self) (`KismetMathLibrary.Conv_VectorToTransform` (+ _returnvalue_location (`KismetMathLibrary.MakeVector` (`self.distence`)))) "Undefined" "MultiplyWithRoot" null null))
      (bind _output_get (set `self.BP_Object` _returnvalue))
      (`self.SetActorHiddenInGame` _output_get false)
      (bind _can (`self.bianjie`))
      (if _can
        (`self.K2_AddActorWorldOffset` (`KismetMathLibrary.MakeVector` (`self.distence`))))
      (`self.K2_DestroyActor` (`self.BP_Object`)))))

(event `Key|A`
  (params (Key :type "Key Structure"))
  (bind _returnvalue_location (`KismetMathLibrary.BreakTransform` (`self.GetTransform` self)))
  (:`Pressed`
    (if (not (`self.place`))
      (bind _returnvalue (`|SpawnActorFromClass` (`GameplayStatics.GetObjectClass` self) (`KismetMathLibrary.Conv_VectorToTransform` (+ _returnvalue_location (`KismetMathLibrary.MakeVector` 0.0 (* (`self.distence`) -1.0)))) "Undefined" "MultiplyWithRoot" null null))
      (bind _output_get (set `self.BP_Object` _returnvalue))
      (`self.SetActorHiddenInGame` _output_get false)
      (bind _can (`self.bianjie`))
      (if _can
        (`self.K2_AddActorWorldOffset` (`KismetMathLibrary.MakeVector` 0.0 (* (`self.distence`) -1.0))))
      (`self.K2_DestroyActor` (`self.BP_Object`)))))

(event `Key|S`
  (params (Key :type "Key Structure"))
  (bind _returnvalue_location (`KismetMathLibrary.BreakTransform` (`self.GetTransform` self)))
  (:`Pressed`
    (if (not (`self.place`))
      (bind _returnvalue (`|SpawnActorFromClass` (`GameplayStatics.GetObjectClass` self) (`KismetMathLibrary.Conv_VectorToTransform` (+ _returnvalue_location (`KismetMathLibrary.MakeVector` (* (`self.distence`) -1.0)))) "Undefined" "MultiplyWithRoot" null null))
      (bind _output_get (set `self.BP_Object` _returnvalue))
      (`self.SetActorHiddenInGame` _output_get false)
      (bind _can (`self.bianjie`))
      (if _can
        (`self.K2_AddActorWorldOffset` (`KismetMathLibrary.MakeVector` (* (`self.distence`) -1.0))))
      (`self.K2_DestroyActor` (`self.BP_Object`)))))

(event `Key|D`
  (params (Key :type "Key Structure"))
  (bind _returnvalue_location (`KismetMathLibrary.BreakTransform` (`self.GetTransform` self)))
  (:`Pressed`
    (if (not (`self.place`))
      (bind _returnvalue (`|SpawnActorFromClass` (`GameplayStatics.GetObjectClass` self) (`KismetMathLibrary.Conv_VectorToTransform` (+ _returnvalue_location (`KismetMathLibrary.MakeVector` 0.0 (`self.distence`)))) "Undefined" "MultiplyWithRoot" null null))
      (bind _output_get (set `self.BP_Object` _returnvalue))
      (`self.SetActorHiddenInGame` _output_get false)
      (bind _can (`self.bianjie`))
      (if _can
        (`self.K2_AddActorWorldOffset` (`KismetMathLibrary.MakeVector` 0.0 (`self.distence`))))
      (`self.K2_DestroyActor` (`self.BP_Object`)))))

(fn `bianjie`
  (returns (can :type Boolean))
  (return true))

(fn `UserConstructionScript`
  (`parent.UserConstructionScript`))