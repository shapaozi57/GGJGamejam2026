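; Claw-game item actor that shows two Paper2D flipbooks chosen by MaskIndex and, when Move is set, travels along X on looping timelines.
; BeginPlay starts the timeline at Speed and randomly flips the sprite's rotation; MaskIndex 6 uses a second timeline with random pauses.
; SetLocation starts a 0.01-second timer that snaps the second flipbook to BP_ClawBase's Sphere1 until Finish clears it.
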(event `self.ReceiveBeginPlay`
  (bind (_beginlocation_x _beginlocation_y _beginlocation_z) (`KismetMathLibrary.BreakVector` (`self.beginlocation`)))
  (`|ExecutionSequence`
    (:`then_0`
      (`TimelineComponent.SetPlayRate` (`self.时间轴`) (`self.speed`))
      (set `self.beginlocation` (`self.K2_GetActorLocation` self))
      (bind _returnvalue (`GameplayStatics.GetActorOfClass` "/Game/BulePrint/Claw/ClawBase/BP_ClawBase.BP_ClawBase_C"))
      (set `self.BP_Base` _returnvalue)
      (if (`self.move`)
        (if (== (`self.MaskIndex`) 6)
          (`self.play`)
          (else
            (`self.setTIme`)
            (bind (_direction `_新建轨道_0`) (`Timeline|时间轴` :`NewTime` (`KismetMathLibrary.RandomFloatInRange` 0.0 4.0) :!label _label)
              (:`Update`
                (`self.K2_SetActorLocation` (`KismetMathLibrary.MakeVector` (* `_新建轨道_0` (`self.length`)) _beginlocation_y _beginlocation_z)))
              (:`Finished`
                (goto _label :!via `PlayFromStart`)))))))
    (:`then_1`
      (if (not (`KismetMathLibrary.RandomBool`))
        (`SceneComponent.K2_SetWorldRotation` (`self.PaperFlipbook`) (struct :`Yaw` 270.0 :`Roll` 90.0) false false)))))

(event `setTIme`
  (goto _label :!via `SetNewTime`))

(event `play`
  (bind (_beginlocation_x _beginlocation_y _beginlocation_z) (`KismetMathLibrary.BreakVector` (`self.beginlocation`)))
  (bind (_direction `_新建轨道_0`) (`Timeline|时间轴_0` :!label _label_2)
    (:`Update`
      (`self.K2_SetActorLocation` (`KismetMathLibrary.MakeVector` (* `_新建轨道_0` (`self.length`)) _beginlocation_y _beginlocation_z)))
    (:`Finished`
      (if (< (`KismetMathLibrary.RandomFloatInRange` 0.0 (`self.gailv`)) 0.5)
        (`self.stopEvent`)
        (else
          (goto _label_2 :!via `PlayFromStart`))))))

(event `stop`
  (goto _label_2 :!via `Stop`))

(event `stopEvent`
  (`self.play`)
  (`KismetSystemLibrary.Delay` (`KismetMathLibrary.RandomFloatInRange` 0.0 3.0))
  (`self.stop`)
  (`KismetSystemLibrary.Delay` (`self.DalayTime`))
  (`self.play`))

(fn `Finish`
  (`KismetSystemLibrary.K2_ClearAndInvalidateTimerHandle` (`self.Timer`)))

(fn `SetLocation`
  (bind _returnvalue (`KismetSystemLibrary.K2_SetTimer` null "Update" 0.01 true))
  (set `self.Timer` _returnvalue))

(fn `Update`
  (`SceneComponent.K2_SetWorldLocation` (`self.PaperFlipbook1`) (`SceneComponent.K2_GetComponentLocation` (`/Game/BulePrint/Claw/ClawBase/BP_ClawBase.Sphere1` (`self.BP_Base`))) false false))

(fn `UserConstructionScript`
  (bind _paperflipbook (`self.PaperFlipbook`))
  (`SceneComponent.SetRelativeScale3D` (`self.Cone`) (`self.scale`))
  (switch `int` (`self.MaskIndex`)
    (:`Default`
      (`PaperFlipbookComponent.SetFlipbook` (`self.PaperFlipbook1`) "/Game/Art/miniMask/FB_UntitledArtwork31__1___2___1___1__-_Reference_Layer_1_-_4-2_0.FB_UntitledArtwork31__1___2___1___1__-_Reference_Layer_1_-_4-2_0" :!label _label)
      (`PaperFlipbookComponent.SetFlipbook` _paperflipbook "/Game/Art/dancer/a.a"))
    (:`0`
      (goto _label))
    (:`1`
      (`PaperFlipbookComponent.SetFlipbook` (`self.PaperFlipbook1`) "/Game/Art/miniMask/FB_UntitledArtwork31__1___2___1___1__-_Reference_Layer_1_-_4-5_0.FB_UntitledArtwork31__1___2___1___1__-_Reference_Layer_1_-_4-5_0")
      (`PaperFlipbookComponent.SetFlipbook` _paperflipbook "/Game/Art/dancer/c.c"))
    (:`2`
      (`PaperFlipbookComponent.SetFlipbook` (`self.PaperFlipbook1`) "/Game/Art/miniMask/FB_UntitledArtwork31__1___2___1___1__-_Reference_Layer_1_-_4-3_0.FB_UntitledArtwork31__1___2___1___1__-_Reference_Layer_1_-_4-3_0")
      (`PaperFlipbookComponent.SetFlipbook` _paperflipbook "/Game/Art/dancer/c.c"))
    (:`3`
      (`PaperFlipbookComponent.SetFlipbook` (`self.PaperFlipbook1`) "/Game/Art/miniMask/FB_UntitledArtwork31__1___2___1___1__-_Reference_Layer_1_-_4-1_0.FB_UntitledArtwork31__1___2___1___1__-_Reference_Layer_1_-_4-1_0")
      (`PaperFlipbookComponent.SetFlipbook` _paperflipbook "/Game/Art/dancer/UnatitledArtwork31__1___2___1___1__-_Group_4__3__-_1.UnatitledArtwork31__1___2___1___1__-_Group_4__3__-_1"))
    (:`4`
      (`PaperFlipbookComponent.SetFlipbook` (`self.PaperFlipbook1`) "/Game/Art/miniMask/FB_UntitledArtwork31__1___2___1___1__-_Reference_Layer_1_-_4-4_0.FB_UntitledArtwork31__1___2___1___1__-_Reference_Layer_1_-_4-4_0")
      (`PaperFlipbookComponent.SetFlipbook` _paperflipbook "/Game/Art/dancer/UnatitledArtwork31__1___2___1___1__-_Group_4__3__-_1.UnatitledArtwork31__1___2___1___1__-_Group_4__3__-_1"))
    (:`5`
      (`PaperFlipbookComponent.SetFlipbook` (`self.PaperFlipbook1`) "/Game/Art/miniMask/FB_UntitledArtwork31__1___2___1___1__-_Reference_Layer_1_-_4-6_0.FB_UntitledArtwork31__1___2___1___1__-_Reference_Layer_1_-_4-6_0")
      (`PaperFlipbookComponent.SetFlipbook` _paperflipbook "/Game/Art/dancer/UntitledArtwork31__1___2___1___1__-_Group_4__3__-_1.UntitledArtwork31__1___2___1___1__-_Group_4__3__-_1"))))