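; Player-controlled puzzle piece made of BP_Puzzle_Unit child actors, placed on a BP_EmptyGrid board for score.
; Outside claw mode, keys step, rotate or delete it, validating moves by spawning a temporary copy to test grid overlap.
; Each unit's nearest overlapping cell decides placeability, shown as yellow or red.
; Space triggers the claw in claw mode; otherwise it fills cells, locks the piece green, adds score, restores claw mode and runs EndCheck.
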(event `self.ReceiveBeginPlay`
  (`|ExecutionSequence`
    (:`then_0`
      (`self.EnableInput` (`GameplayStatics.GetPlayerController` 0)))
    (:`then_1`
      (for _array_element (`self.GetAllChildActors` true)
        (bind _asbp_puzzle_unit (cast `/Game/BulePrint/RightScene/BP_Puzzle_Unit` _array_element))
        (`KismetArrayLibrary.Array_Add` (`self.Units`) _asbp_puzzle_unit)
        (`self.CheckCanPutIn`)))))

(event `Key|P`
  (params (Key :type "Key Structure"))
  (:`Pressed`
    (`KismetSystemLibrary.PrintString` "Hello")
    (bind _astestgamemode (cast `/Game/BulePrint/testgamemode` (`GameplayStatics.GetGameMode`)))
    (`/Game/BulePrint/testgamemode.EndLevel` _astestgamemode)))

(event `Key|Up`
  (params (Key :type "Key Structure"))
  (bind _defaultsceneroot (`self.DefaultSceneRoot`))
  (bind _returnvalue (`SceneComponent.K2_GetComponentToWorld` (`self.DefaultSceneRoot`)))
  (bind (_returnvalue_x _returnvalue_y _returnvalue_z) (`KismetMathLibrary.BreakVector` (`SceneComponent.K2_GetComponentLocation` _defaultsceneroot)))
  ;[1 1 1] controll
  (:`Pressed`
    (`self.ModeCheckNotClaw`)
    (`self.MoveCheck` (`KismetMathLibrary.MakeTransform` (`KismetMathLibrary.MakeVector` (+ (.x (.location _returnvalue)) 65.0) (.y (.location _returnvalue)) (.z (.location _returnvalue))) (.rotation _returnvalue) (.scale _returnvalue)))
    (if (and (`self.IsActiveGroup`) (`self.CanMove`))
      (`SceneComponent.K2_SetWorldLocation` _defaultsceneroot (`KismetMathLibrary.MakeVector` (+ _returnvalue_x 65.0) _returnvalue_y _returnvalue_z) false false)
      (`self.CheckCanPutIn` :!label _label))))

(event `Key|D`
  (params (Key :type "Key Structure"))
  (bind _defaultsceneroot (`self.DefaultSceneRoot`))
  (bind _returnvalue (`SceneComponent.K2_GetComponentToWorld` (`self.DefaultSceneRoot`)))
  (bind (_returnvalue_roll _returnvalue_pitch _returnvalue_yaw) (`KismetMathLibrary.BreakRotator` (`SceneComponent.K2_GetComponentRotation` _defaultsceneroot)))
  ;[1 1 1] rotate
  (:`Pressed`
    (`self.ModeCheckNotClaw`)
    (`self.RotateCheck` (`KismetMathLibrary.MakeTransform` (.location _returnvalue) (`KismetMathLibrary.MakeRotator` (.roll (.rotation _returnvalue)) (.pitch (.rotation _returnvalue)) (- (.yaw (.rotation _returnvalue)) 90.0)) (.scale _returnvalue)))
    (if (and (`self.IsActiveGroup`) (`self.CanMove`))
      (`SceneComponent.K2_SetWorldRotation` _defaultsceneroot (`KismetMathLibrary.MakeRotator` _returnvalue_roll _returnvalue_pitch (- _returnvalue_yaw 90.0)) false false)
      (`self.CheckCanPutIn`))))

(event `Key|Down`
  (params (Key :type "Key Structure"))
  (bind _defaultsceneroot (`self.DefaultSceneRoot`))
  (bind _returnvalue (`SceneComponent.K2_GetComponentToWorld` (`self.DefaultSceneRoot`)))
  (bind (_returnvalue_x _returnvalue_y _returnvalue_z) (`KismetMathLibrary.BreakVector` (`SceneComponent.K2_GetComponentLocation` _defaultsceneroot)))
  ;[1 1 1] controll
  (:`Pressed`
    (`self.ModeCheckNotClaw`)
    (`self.MoveCheck` (`KismetMathLibrary.MakeTransform` (`KismetMathLibrary.MakeVector` (- (.x (.location _returnvalue)) 65.0) (.y (.location _returnvalue)) (.z (.location _returnvalue))) (.rotation _returnvalue) (.scale _returnvalue)))
    (if (and (`self.IsActiveGroup`) (`self.CanMove`))
      (`SceneComponent.K2_SetWorldLocation` _defaultsceneroot (`KismetMathLibrary.MakeVector` (- _returnvalue_x 65.0) _returnvalue_y _returnvalue_z) false false)
      (goto _label))))

(event `RotateCheck`
  (params (Rotation :type "Transform Structure"))
  ;[1 1 1] rotate
  (bind _returnvalue (`|SpawnActorFromClass` (`GameplayStatics.GetObjectClass` self) Rotation "Undefined" "MultiplyWithRoot" null null))
  (`self.checkCanMove` _returnvalue)
  (if (`/Game/BulePrint/RightScene/BP_Puzzle_Group.CanMove` _returnvalue)
    (set `self.CanMove` true)
    (else
      (set `self.CanMove` false)))
  (`KismetSystemLibrary.PrintString` (`KismetStringLibrary.Conv_BoolToString` (`self.CanMove`)))
  (`self.K2_DestroyActor` _returnvalue))

(event `Key|Left`
  (params (Key :type "Key Structure"))
  (bind _defaultsceneroot (`self.DefaultSceneRoot`))
  (bind _returnvalue (`SceneComponent.K2_GetComponentToWorld` (`self.DefaultSceneRoot`)))
  (bind (_returnvalue_x _returnvalue_y _returnvalue_z) (`KismetMathLibrary.BreakVector` (`SceneComponent.K2_GetComponentLocation` _defaultsceneroot)))
  ;[1 1 1] controll
  (:`Pressed`
    (`self.ModeCheckNotClaw`)
    (`self.MoveCheck` (`KismetMathLibrary.MakeTransform` (`KismetMathLibrary.MakeVector` (.x (.location _returnvalue)) (- (.y (.location _returnvalue)) 65.0) (.z (.location _returnvalue))) (.rotation _returnvalue) (.scale _returnvalue)))
    (if (and (`self.IsActiveGroup`) (`self.CanMove`))
      (`SceneComponent.K2_SetWorldLocation` _defaultsceneroot (`KismetMathLibrary.MakeVector` _returnvalue_x (- _returnvalue_y 65.0) _returnvalue_z) false false)
      (goto _label))))

(event `Key|Right`
  (params (Key :type "Key Structure"))
  (bind _defaultsceneroot (`self.DefaultSceneRoot`))
  (bind _returnvalue (`SceneComponent.K2_GetComponentToWorld` (`self.DefaultSceneRoot`)))
  (bind (_returnvalue_x _returnvalue_y _returnvalue_z) (`KismetMathLibrary.BreakVector` (`SceneComponent.K2_GetComponentLocation` _defaultsceneroot)))
  ;[1 1 1] controll
  (:`Pressed`
    (`self.ModeCheckNotClaw`)
    (`self.MoveCheck` (`KismetMathLibrary.MakeTransform` (`KismetMathLibrary.MakeVector` (.x (.location _returnvalue)) (+ (.y (.location _returnvalue)) 65.0) (.z (.location _returnvalue))) (.rotation _returnvalue) (.scale _returnvalue)))
    (if (and (`self.IsActiveGroup`) (`self.CanMove`))
      (`SceneComponent.K2_SetWorldLocation` _defaultsceneroot (`KismetMathLibrary.MakeVector` _returnvalue_x (+ _returnvalue_y 65.0) _returnvalue_z) false false)
      (goto _label))))

(event `Key|SpaceBar`
  (params (Key :type "Key Structure"))
  (bind _choosecloseestunit (`self.ChooseCloseestUnit`))
  (bind _defaultsceneroot (`self.DefaultSceneRoot`))
  (bind (_returnvalue_x _returnvalue_y) (`KismetMathLibrary.BreakVector` (`SceneComponent.K2_GetComponentLocation` _defaultsceneroot)))
  ;[1 1 1] putin
  (:`Pressed`
    (`KismetSystemLibrary.PrintString` "Hello")
    (bind _astestgamemode (cast `/Game/BulePrint/testgamemode` (`GameplayStatics.GetGameMode`)))
    (if (`/Game/BulePrint/testgamemode.IsClawMode` _astestgamemode)
      (bind _returnvalue (`GameplayStatics.GetActorOfClass` "/Game/BulePrint/Claw/ClawBase/BP_ClawBase.BP_ClawBase_C"))
      (`/Game/BulePrint/Claw/ClawBase/BP_ClawBase.claw` _returnvalue)
      (elif (`self.CanPutIn`)
        (for _array_element (`self.Units`)
          (set `self.ChooseCloseestUnit` null)
          (set `self.tempDistance` 0.0)
          (for _array_element_2 (`PrimitiveComponent.GetOverlappingActors` (`/Game/BulePrint/RightScene/BP_Puzzle_Unit.Box` _array_element) "/Game/BulePrint/RightScene/BP_EmptyGrid.BP_EmptyGrid_C")
            (if (== (`self.tempDistance`) 0.0)
              (bind _returnvalue_2 (`self.GetDistanceTo` _array_element _array_element_2))
              ;;[1 1 1] first time sign up
              (set `self.tempDistance` _returnvalue_2)
              (set `self.ChooseCloseestUnit` _array_element_2)
              (else
                ;;[1 1 1] overwrite closest
                (if (< _returnvalue_2 (`self.tempDistance`))
                  (set `self.tempDistance` _returnvalue_2)
                  (set `self.ChooseCloseestUnit` _array_element_2)))))
          (`/Engine/EditorBlueprintResources/StandardMacros.IsValid` _choosecloseestunit
            (:`Is Valid`
              (bind _asbp_empty_grid (cast `/Game/BulePrint/RightScene/BP_EmptyGrid` _choosecloseestunit))
              (set `/Game/BulePrint/RightScene/BP_EmptyGrid.UnFilled` false _asbp_empty_grid))))
        (`KismetSystemLibrary.PrintString` "Succeed")
        (`SceneComponent.K2_SetWorldLocation` _defaultsceneroot (`KismetMathLibrary.MakeVector` _returnvalue_x _returnvalue_y 10.0) false false)
        (set `self.IsActiveGroup` false)
        (for _array_element_3 (`self.Units`)
          (`PaperFlipbookComponent.SetSpriteColor` (`/Game/BulePrint/RightScene/BP_Puzzle_Unit.PaperFlipbook` _array_element_3) (struct :`R` 0.32675 :`G` 0.742188 :`B` 0.149306 :`A` 1.0)))
        ;;[1 1 1] reset and switch mode
        (bind _astestgamemode_2 (cast `/Game/BulePrint/testgamemode` (`GameplayStatics.GetGameMode`)))
        (set `/Game/BulePrint/testgamemode.CollectedMaskIndex` -1 _astestgamemode_2)
        (set `/Game/BulePrint/testgamemode.IsClawMode` true _astestgamemode_2)
        (`self.AddScore`)
        (`/Game/BulePrint/testgamemode.EndCheck` _astestgamemode_2)
        (else
          (`KismetSystemLibrary.PrintString` "Failed"))))))

(event `Key|F`
  (params (Key :type "Key Structure"))
  ;[1 1 1] delete
  (:`Pressed`
    (`self.ModeCheckNotClaw`)
    (`self.K2_DestroyActor`)
    (bind _astestgamemode (cast `/Game/BulePrint/testgamemode` (`GameplayStatics.GetGameMode`)))
    (set `/Game/BulePrint/testgamemode.CollectedMaskIndex` -1 _astestgamemode)
    (set `/Game/BulePrint/testgamemode.IsClawMode` true _astestgamemode)
    (`/Game/BulePrint/testgamemode.EndCheck` _astestgamemode)))

(event `CheckCanPutIn`
  (bind _choosecloseestunit (`self.ChooseCloseestUnit`))
  ;[1 1 1] show red green
  (for _array_element (`self.Units`)
    (set `self.ChooseCloseestUnit` null)
    (set `self.tempDistance` 0.0)
    (for _array_element_2 (`PrimitiveComponent.GetOverlappingActors` (`/Game/BulePrint/RightScene/BP_Puzzle_Unit.Box` _array_element) "/Game/BulePrint/RightScene/BP_EmptyGrid.BP_EmptyGrid_C")
      (if (== (`self.tempDistance`) 0.0)
        (bind _returnvalue (`self.GetDistanceTo` _array_element _array_element_2))
        ;;[1 1 1] first time sign up
        (set `self.tempDistance` _returnvalue)
        (set `self.ChooseCloseestUnit` _array_element_2)
        (else
          ;;[1 1 1] overwrite closest
          (if (< _returnvalue (`self.tempDistance`))
            (set `self.tempDistance` _returnvalue)
            (set `self.ChooseCloseestUnit` _array_element_2)))))
    (`/Engine/EditorBlueprintResources/StandardMacros.IsValid` _choosecloseestunit
      (:`Is Valid`
        (bind _asbp_empty_grid (cast `/Game/BulePrint/RightScene/BP_EmptyGrid` _choosecloseestunit))
        (if (and (`/Game/BulePrint/RightScene/BP_EmptyGrid.Avaliable` _asbp_empty_grid) (`/Game/BulePrint/RightScene/BP_EmptyGrid.UnFilled` _asbp_empty_grid))
          (set `self.CanPutIn` true)
          (else
            (set `self.CanPutIn` false :!label _label_2)
            (break))))
      (:`Is Not Valid`
        (goto _label_2))))
  ;;[1 1 1] set color
  (if (`self.CanPutIn`)
    (for _array_element_3 (`self.Units`)
      (`PaperFlipbookComponent.SetSpriteColor` (`/Game/BulePrint/RightScene/BP_Puzzle_Unit.PaperFlipbook` _array_element_3) (struct :`R` 0.742188 :`G` 0.731446 :`B` 0.172017 :`A` 1.0)))
    (else
      (for _array_element_4 (`self.Units`)
        (`PaperFlipbookComponent.SetSpriteColor` (`/Game/BulePrint/RightScene/BP_Puzzle_Unit.PaperFlipbook` _array_element_4) (struct :`R` 0.609375 :`G` 0.114258 :`B` 0.114258 :`A` 1.0))))))

(event `AddScore`
  (bind _foundwidgets (`WidgetBlueprintLibrary.GetAllWidgetsOfClass` "/Game/Widget/UI_InGame.UI_InGame_C"))
  (for _array_element _foundwidgets
    (`/Game/Widget/UI_InGame.addWithFloat` _array_element (`self.Score`))
    (`GameplayStatics.PlaySound2D` "/Game/sound/money.money" 1.0 1.0 0.0 null null)))

(event `BonusCheck`
  (`|ExecutionSequence`))

(event `MoveCheck`
  (params (TargetLocation :type "Transform Structure"))
  ;[1 1 1] checkCanMove
  (bind _returnvalue (`|SpawnActorFromClass` (`GameplayStatics.GetObjectClass` self) TargetLocation "Undefined" "MultiplyWithRoot" null null))
  (`self.checkCanMove` _returnvalue)
  (if (`/Game/BulePrint/RightScene/BP_Puzzle_Group.CanMove` _returnvalue)
    (set `self.CanMove` true)
    (else
      (set `self.CanMove` false)))
  (`self.K2_DestroyActor` _returnvalue))

(event `checkCanMove`
  ;[1 1 1] checkCanMove
  (for _array_element (`self.Units`)
    (set `self.ChooseCloseestUnit` null)
    (set `self.tempDistance` 0.0)
    (for _array_element_2 (`PrimitiveComponent.GetOverlappingActors` (`/Game/BulePrint/RightScene/BP_Puzzle_Unit.Box` _array_element) "/Game/BulePrint/RightScene/BP_EmptyGrid.BP_EmptyGrid_C")
      (if (== (`self.tempDistance`) 0.0)
        (bind _returnvalue (`self.GetDistanceTo` _array_element _array_element_2))
        ;;[1 1 1] first time sign up
        (set `self.tempDistance` _returnvalue)
        (set `self.ChooseCloseestUnit` _array_element_2)
        (else
          ;;[1 1 1] overwrite closest
          (if (< _returnvalue (`self.tempDistance`))
            (set `self.tempDistance` _returnvalue)
            (set `self.ChooseCloseestUnit` _array_element_2)))))
    (`/Engine/EditorBlueprintResources/StandardMacros.IsValid` (`self.ChooseCloseestUnit`)
      (:`Is Valid`
        (set `self.CanMove` true))
      (:`Is Not Valid`
        (set `self.CanMove` false)
        (break)))))

(fn `UserConstructionScript`)