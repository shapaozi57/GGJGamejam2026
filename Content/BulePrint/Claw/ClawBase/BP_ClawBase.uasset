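; BP_ClawBase is a swinging claw that grabs BP_object items, in the style of Gold Miner.
; A looping timer swings it until claw() fires, when a timeline extends and retracts the head while scaling the rod to match.
; Overlapping an item starts retraction at a speed set by Power and Weight.
; On return, MaskIndex selects repositioning the item's flipbook, opening Level1, or passing the mask to testgamemode for a new puzzle.
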(event `claw`
  (bind _as_bp_object (`self.As BP Object`))
  (bind _as_bp_object_2 (`self.As BP Object`))
  (bind _arrow (`self.arrow`))
  ;[1 0.1094 0.2242] spacebar
  (`self.DisableInput` (`GameplayStatics.GetPlayerController` 0))
  (`KismetSystemLibrary.K2_ClearAndInvalidateTimerHandle` (`self.RotationHandle`))
  (bind (_direction `_新建轨道_0`) (`Timeline|时间轴` :!label _label)
    (:`Update`
      (`SceneComponent.K2_SetWorldLocation` (`self.Sphere1`) (+ (`SceneComponent.K2_GetComponentLocation` _arrow) (* (`SceneComponent.GetForwardVector` _arrow) `_新建轨道_0`)) false false)
      (`SceneComponent.SetRelativeScale3D` (`self.gan`) (`KismetMathLibrary.MakeVector` 1.0 1.0 (/ (`KismetMathLibrary.Vector_Distance` (`SceneComponent.K2_GetComponentLocation` (`self.Sphere`)) (`SceneComponent.K2_GetComponentLocation` (`self.Sphere1`))) 21.0))))
    (:`Finished`
      (if (== `_新建轨道_0` 0.0)
        (`self.EnableInput` (`GameplayStatics.GetPlayerController` 0))
        (bind _returnvalue (`KismetSystemLibrary.K2_SetTimerDelegate` (`|CreateDelegate` :!event `Rota`) 0.01 true))
        (set `self.RotationHandle` _returnvalue)
        (`/Engine/EditorBlueprintResources/StandardMacros.IsValid` _as_bp_object_2
          (:`Is Valid`
            (if (== (`/Game/BulePrint/Item/BP_object.MaskIndex` (`self.As BP Object`)) 6)
              (`SceneComponent.K2_SetWorldLocation` (`/Game/BulePrint/Item/BP_object.PaperFlipbook1` _as_bp_object_2) (`SceneComponent.K2_GetComponentLocation` (`/Game/BulePrint/Item/BP_object.PaperFlipbook` _as_bp_object_2)) false false)
              (set `self.As BP Object` null)
              (`TimelineComponent.SetPlayRate` (`self.时间轴`) 1.0)
              (elif (== (`/Game/BulePrint/Item/BP_object.MaskIndex` (`self.As BP Object`)) 7)
                (`GameplayStatics.OpenLevel` "Level1")
                (else
                  (bind _astestgamemode (cast `/Game/BulePrint/testgamemode` (`GameplayStatics.GetGameMode`)))
                  (set `/Game/BulePrint/testgamemode.CollectedMaskIndex` (`/Game/BulePrint/Item/BP_object.MaskIndex` (`self.As BP Object`)) _astestgamemode)
                  (`/Game/BulePrint/testgamemode.SpawnNewPuzzle` _astestgamemode)
                  (set `/Game/BulePrint/testgamemode.IsClawMode` false _astestgamemode)
                  (`self.SetActorEnableCollision` _as_bp_object false)
                  (`SceneComponent.SetVisibility` (`/Game/BulePrint/Item/BP_object.PaperFlipbook1` _as_bp_object) false false)
                  (set `self.As BP Object` null)
                  (`TimelineComponent.SetPlayRate` (`self.时间轴`) 1.0))))))
        (else
          (`self.RePlay`))))))

(event `RePlay`
  ;[1 0.1094 0.2242] spacebar
  (goto _label :!via `Reverse`))

(event `self.ReceiveBeginPlay`
  ;[1 0.3322 0.1024] begin
  (set `self.cishu` 0)
  (`SceneComponent.SetRelativeScale3D` (`self.gan`) (`KismetMathLibrary.MakeVector` 1.0 1.0 (/ (`KismetMathLibrary.Vector_Distance` (`SceneComponent.K2_GetComponentLocation` (`self.Sphere`)) (`SceneComponent.K2_GetComponentLocation` (`self.Sphere1`))) 20.0)))
  (`self.EnableInput` (`GameplayStatics.GetPlayerController` 0))
  (bind _returnvalue (`KismetSystemLibrary.K2_SetTimerDelegate` (`|CreateDelegate` :!event `Rota`) 0.01 true))
  (set `self.RotationHandle` _returnvalue))

(event `self.Sphere2.OnComponentBeginOverlap`
  (params (OverlappedComponent :type "PrimitiveComponent Object Reference") (OtherActor :type "Actor Object Reference") (OtherComp :type "PrimitiveComponent Object Reference") (OtherBodyIndex :type Integer) (bFromSweep :type Boolean) (SweepResult :type "HitResult Structure (by ref)"))
  (bind _paperflipbook3 (`self.PaperFlipbook3`))
  ;[1 0.6324 0] collision
  (set `self.cishu` (+ (`self.cishu`) 1))
  (bind _returnvalue (`GameplayStatics.GetCurrentLevelName` true))
  (if (and (== (`KismetStringLibrary.Conv_StringToName` _returnvalue) "Level1") (== (`self.cishu`) 1))
    (`SceneComponent.SetHiddenInGame` _paperflipbook3 false false)
    (`KismetSystemLibrary.Delay` 2.0)
    (`SceneComponent.SetHiddenInGame` _paperflipbook3 true false))
  (`/Engine/EditorBlueprintResources/StandardMacros.IsValid` (`self.As BP Object`)
    (:`Is Not Valid`
      (bind _asbp_object (cast `/Game/BulePrint/Item/BP_object` OtherActor))
      (bind _output_get (set `self.As BP Object` _asbp_object))
      (`/Game/BulePrint/Item/BP_object.SetLocation` _output_get)
      (`self.RePlay`)
      (`TimelineComponent.SetPlayRate` (`self.时间轴`) (/ 1.0 (/ (`/Game/BulePrint/Item/BP_object.weight` _output_get) (`self.Power`)))))))

(event `Rota`
  (bind _rotatespeed (`self.RotateSpeed`))
  (bind _sphere (`self.Sphere`))
  (bind (_returnvalue_roll _returnvalue_pitch _returnvalue_yaw) (`KismetMathLibrary.BreakRotator` (`SceneComponent.K2_GetComponentRotation` (`self.Sphere`))))
  (bind _returnvalue (`KismetMathLibrary.FTrunc` _returnvalue_yaw))
  ;[0.4241 1 0] rotation
  (if (== _returnvalue 120.0)
    (set `self.fan` true))
  (if (== _returnvalue -120)
    (set `self.fan` false))
  (if (`self.fan`)
    (`SceneComponent.K2_AddLocalRotation` _sphere (`KismetMathLibrary.MakeRotator` 0.0 (* _rotatespeed -1.0)) false false)
    (else
      (`SceneComponent.K2_AddLocalRotation` _sphere (`KismetMathLibrary.MakeRotator` 0.0 _rotatespeed) false false))))

(fn `UserConstructionScript`)